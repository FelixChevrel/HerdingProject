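; BP_Bait is a physics-driven bait actor that a BP_Dragonfly can carry, apparently toward the player.
; PushTowardPlayer disables physics on its Sphere, attaches the bait to the first dragonfly found at its current world transform, and binds Drop to that dragonfly's CameBack event.
; Drop re-enables physics without an explicit detach, then clears every CameBack binding on the first dragonfly found, not just its own.
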(event `/Game/Interface/BPI_DragonflyInteraction.PushTowardPlayer`
  (bind _outactors (`GameplayStatics.GetAllActorsOfClass` "/Game/Creatures/DragonFly/BP_Dragonfly.BP_Dragonfly_C"))
  (`PrimitiveComponent.SetSimulatePhysics` (`self.Sphere`) false)
  (bind _output (`|GetArrayItem` _outactors))
  (`self.K2_AttachToActor` _output "None" "KeepWorld" "KeepWorld" "KeepWorld")
  (add `/Game/Creatures/DragonFly/BP_Dragonfly.CameBack` _output (delegate `Drop`)))

(event `Drop`
  (`PrimitiveComponent.SetSimulatePhysics` (`self.Sphere`) true)
  (bind _outactors (`GameplayStatics.GetAllActorsOfClass` "/Game/Creatures/DragonFly/BP_Dragonfly.BP_Dragonfly_C"))
  (clear `/Game/Creatures/DragonFly/BP_Dragonfly.CameBack` (`|GetArrayItem` _outactors)))

(fn `UserConstructionScript`)