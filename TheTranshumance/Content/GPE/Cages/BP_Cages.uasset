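; BP_Cages is a cage prop that breaks apart when hit.
; GetHit swaps the static mesh for a hidden Geometry Collection at the same transform, enables its physics and applies an impulse at the hit point along the hit direction.
; After a short delay, the FinishDesintegrate timeline animates the debris scale, then the actor is destroyed.
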(event `/Game/GPE/BPI_StrikeInteraction.GetHit`
  (params (Hitcoordinate :type "Vector Structure") (ForwardVector :type "Vector Structure"))
  (bind _geometrycollection (`self.GeometryCollection`))
  (bind _staticmesh (`self.StaticMesh`))
  (`SceneComponent.K2_SetWorldTransform` _geometrycollection (`SceneComponent.K2_GetComponentToWorld` _staticmesh) false false)
  (`ActorComponent.K2_DestroyComponent` _staticmesh)
  (`SceneComponent.SetVisibility` _geometrycollection true false)
  (`PrimitiveComponent.SetCollisionEnabled` _geometrycollection "QueryAndPhysics")
  (`PrimitiveComponent.SetSimulatePhysics` _geometrycollection true)
  (`PrimitiveComponent.AddImpulseAtLocation` _geometrycollection (* ForwardVector 500.0) Hitcoordinate "None")
  (`KismetSystemLibrary.Delay` 4.0)
  (bind (_direction _newtrack_0) (`Timeline|FinishDesintegrate`)
    (:`Update`
      (`SceneComponent.SetWorldScale3D` (`self.GeometryCollection`) (`KismetMathLibrary.MakeVector` _newtrack_0 _newtrack_0 _newtrack_0)))
    (:`Finished`
      (`self.K2_DestroyActor`))))

(fn `UserConstructionScript`)