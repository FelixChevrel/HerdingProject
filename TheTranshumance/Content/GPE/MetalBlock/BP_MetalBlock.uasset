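; BP_MetalBlock is a block that gets shoved along a grid-aligned direction when hit.
; Each tick, CenterArrow's yaw snaps to the nearest 90 degrees toward the player.
; GetHit sweeps the mesh along Arrow's forward vector via a sped-up timeline with a vertical arc, travelling less at larger scales.
; A DoOnce blocks further hits until a short delay after the move ends.
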(event `self.ReceiveBeginPlay`
  (`TimelineComponent.SetPlayRate` (`self.Push2mForward`) 5.0))

(event `self.ReceiveTick`
  (params (DeltaSeconds :type "Float (single-precision)"))
  (bind (_returnvalue_roll _returnvalue_pitch _returnvalue_yaw) (`KismetMathLibrary.BreakRotator` (`KismetMathLibrary.FindLookAtRotation` (`self.K2_GetActorLocation`) (`self.K2_GetActorLocation` (`GameplayStatics.GetPlayerPawn` 0)))))
  (`SceneComponent.K2_SetWorldRotation` (`self.CenterArrow`) (`KismetMathLibrary.MakeRotator` 0.0 0.0 (`self.GetCorrectDirection` _returnvalue_yaw)) false false))

(event `/Game/Interface/BPI_StrikeInteraction.GetHit`
  (params (Hitcoordinate :type "Vector Structure") (ForwardVector :type "Vector Structure"))
  (bind _returnvalue_x (`KismetMathLibrary.BreakVector` (`SceneComponent.K2_GetComponentScale` (`self.StaticMesh`))))
  (`/Engine/EditorBlueprintResources/StandardMacros.DoOnce` false :!label _label
    (:`Completed`
      (bind _output_get (set `self.StartGoal` (`self.K2_GetActorLocation`)))
      (set `self.EndGoal` (+ _output_get (* (`SceneComponent.GetForwardVector` (`self.Arrow`)) (/ 200.0 (`KismetMathLibrary.Conv_IntToDouble` (`KismetMathLibrary.Round` _returnvalue_x))))))
      (bind (_direction _newtrack_0 _zarc) (`Timeline|Push2mForward` :!via `PlayFromStart`)
        (:`Update`
          (`SceneComponent.K2_SetWorldLocation` (`self.StaticMesh`) (+ (`KismetMathLibrary.VLerp` (`self.StartGoal`) (`self.EndGoal`) _newtrack_0) (`KismetMathLibrary.MakeVector` 0.0 0.0 _zarc)) true false))
        (:`Finished`
          (`KismetSystemLibrary.Delay` 1.0)
          (goto _label :!via `Reset`))))))

(fn `GetCorrectDirection`
  (params (Value :type "Float (double-precision)"))
  (returns (Return :type "Float (double-precision)"))
  (bind _returnvalue (`KismetMathLibrary.Round` (/ Value 90.0)))
  (return (`KismetMathLibrary.SelectFloat` 180.0 (`KismetMathLibrary.SelectFloat` -90.0 (`KismetMathLibrary.SelectFloat` 0.0 90.0 (== _returnvalue 0)) (== _returnvalue -1)) (or (== _returnvalue -2) (== _returnvalue 2)))))

(fn `UserConstructionScript`)