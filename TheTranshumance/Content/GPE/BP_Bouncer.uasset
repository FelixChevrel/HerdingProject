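; BP_Bouncer is a bounce pad that launches actors implementing BPI_Bouncer when they touch its box.
; On box overlap with an actor's root component, it sends that actor a BOUNCE interface message with the Arrow's forward direction, the Power variable and a short delay, leaving the launch itself to the receiver.
; A Squash timeline then animates the cube's vertical scale as visual feedback.
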(event `self.Box.OnComponentBeginOverlap`
  (params (OverlappedComponent :type "PrimitiveComponent Object Reference") (OtherActor :type "Actor Object Reference") (OtherComp :type "PrimitiveComponent Object Reference") (OtherBodyIndex :type Integer) (bFromSweep :type Boolean) (SweepResult :type "HitResult Structure (by ref)"))
  (if (== OtherComp (`Actor.RootComponent` OtherActor))
    (if (`KismetSystemLibrary.DoesImplementInterface` OtherActor "/Game/Interface/BPI_Bouncer.BPI_Bouncer_C")
      (message `/Game/Interface/BPI_Bouncer.BOUNCE` OtherActor 0.2 (`SceneComponent.GetForwardVector` (`self.Arrow`)) (`self.Power`))
      (bind (_direction _newtrack_0) (`Timeline|Squash` :!via `PlayFromStart`)
        (:`Update`
          (`SceneComponent.SetRelativeScale3D` (`self.Cube`) (`KismetMathLibrary.MakeVector` 1.0 1.0 _newtrack_0)))))))

(fn `UserConstructionScript`)