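; BP_InsectPen is a pen that counts creatures of one valid class entering and leaving it, and closes its gate when full.
; Box overlaps on a creature's root component raise or lower the count and call Added or Removed.
; Reaching max capacity triggers CloseGate, which plays a timeline once to swing the door pivot shut on yaw.
; The gate has no reopening logic, even if the count later drops.
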(event `CloseGate`
  (`/Engine/EditorBlueprintResources/StandardMacros.DoOnce` false
    (:`Completed`
      (bind (_direction _angle) (`Timeline|CloseDoor`)
        (:`Update`
          (`SceneComponent.K2_SetRelativeRotation` (`self.DoorPivot`) (`KismetMathLibrary.MakeRotator` 0.0 0.0 _angle) false false))))))

(event `self.Box.OnComponentBeginOverlap`
  (params (OverlappedComponent :type "PrimitiveComponent Object Reference") (OtherActor :type "Actor Object Reference") (OtherComp :type "PrimitiveComponent Object Reference") (OtherBodyIndex :type Integer) (bFromSweep :type Boolean) (SweepResult :type "HitResult Structure (by ref)"))
  (bind _currentvalue (`self.CurrentValue`))
  (if (and (== (`GameplayStatics.GetObjectClass` OtherActor) (`self.ValideCreatures`)) (== OtherComp (`Actor.RootComponent` OtherActor)))
    (`/Engine/EditorBlueprintResources/StandardMacros.IncrementInt` _currentvalue
      (:`  `
        (`self.Added`)
        (if (== _currentvalue (`self.MaxCapacity`))
          (`self.CloseGate`))))))

(event `self.Box.OnComponentEndOverlap`
  (params (OverlappedComponent :type "PrimitiveComponent Object Reference") (OtherActor :type "Actor Object Reference") (OtherComp :type "PrimitiveComponent Object Reference") (OtherBodyIndex :type Integer))
  (if (and (== (`self.ValideCreatures`) (`GameplayStatics.GetObjectClass` OtherActor)) (== OtherComp (`Actor.RootComponent` OtherActor)))
    (`/Engine/EditorBlueprintResources/StandardMacros.DecrementInt` (`self.CurrentValue`)
      (:`  `
        (`self.Removed`)))))

(fn `UserConstructionScript`)