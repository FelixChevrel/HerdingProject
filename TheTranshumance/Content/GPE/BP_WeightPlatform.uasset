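; Weight-triggered platform that sinks when enough weight rests on it and rises again when the weight drops below the threshold.
; Box overlaps add or subtract weights queried through BPI_EnvironmentInteraction, counting only root components.
; The Lower timeline plays or reverses to lerp the Cube's relative Z down by LoweredDistance.
; The STUCK event toggles a gate that blocks position updates while the timeline keeps running.
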(event `self.ReceiveBeginPlay`
  (`TimelineComponent.SetPlayRate` (`self.Lower`) (`self.LoweringRate`)))

(event `self.Box.OnComponentBeginOverlap`
  (params (OverlappedComponent :type "PrimitiveComponent Object Reference") (OtherActor :type "Actor Object Reference") (OtherComp :type "PrimitiveComponent Object Reference") (OtherBodyIndex :type Integer) (bFromSweep :type Boolean) (SweepResult :type "HitResult Structure (by ref)"))
  (bind _cube (`self.Cube`))
  (bind (_relativelocation_x _relativelocation_y) (`KismetMathLibrary.BreakVector` (`SceneComponent.RelativeLocation` _cube)))
  (if (== OtherComp (`Actor.RootComponent` OtherActor))
    (if (`KismetSystemLibrary.DoesImplementInterface` OtherActor "/Game/Interface/BPI_EnvironmentInteraction.BPI_EnvironmentInteraction_C")
      (bind _weight (message `/Game/Interface/BPI_EnvironmentInteraction.GetWeight` OtherActor))
      (bind _output_get (set `self.CurrentWeight` (+ (`self.CurrentWeight`) _weight)))
      (`KismetSystemLibrary.PrintString` (`KismetStringLibrary.Conv_IntToString` _output_get))
      (if (>= _output_get (`self.ExpectedWeight`))
        (bind (_direction _newtrack_0) (`Timeline|Lower` :!label _label)
          (:`Update`
            (`/Engine/EditorBlueprintResources/StandardMacros.Gate` false :!label _label_2
              (:`Exit`
                (`SceneComponent.K2_SetRelativeLocation` _cube (`KismetMathLibrary.MakeVector` _relativelocation_x _relativelocation_y (`KismetMathLibrary.Lerp` 0.0 (* (`self.LoweredDistance`) -1.0) _newtrack_0)) false false)
                (`KismetSystemLibrary.PrintString` "lower")))))))))

(event `self.Box.OnComponentEndOverlap`
  (params (OverlappedComponent :type "PrimitiveComponent Object Reference") (OtherActor :type "Actor Object Reference") (OtherComp :type "PrimitiveComponent Object Reference") (OtherBodyIndex :type Integer))
  (if (== OtherComp (`Actor.RootComponent` OtherActor))
    (if (`KismetSystemLibrary.DoesImplementInterface` OtherActor "/Game/Interface/BPI_EnvironmentInteraction.BPI_EnvironmentInteraction_C")
      (bind _weight (message `/Game/Interface/BPI_EnvironmentInteraction.GetWeight` OtherActor))
      (bind _output_get (set `self.CurrentWeight` (- (`self.CurrentWeight`) _weight)))
      (`KismetSystemLibrary.PrintString` (`KismetStringLibrary.Conv_IntToString` _output_get))
      (if (not (>= _output_get (`self.ExpectedWeight`)))
        (goto _label :!via `Reverse`)))))

(event `/Game/Interface/BPI_EnvironmentInteraction.STUCK`
  (params (OnOrOff :type Boolean))
  (if OnOrOff
    (goto _label_2 :!via `Close`)
    (else
      (goto _label_2 :!via `Open`))))

(fn `GetWeight`
  (returns (Weight :type Integer))
  (return 0))

(fn `UserConstructionScript`)