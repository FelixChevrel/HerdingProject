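; Bull enemy creature that attacks the player and preys on herd creatures.
; A looping timer checks range, then fires a telegraphed forward sphere trace that stuns the player; EatingRange overlaps start a timeline that lifts and destroys herd creatures.
; Hits stagger it, release prey and drain HitBar; at zero it is stunned, can be launched, and regenerates gradually.
; Tick gates parent behavior, toggles Niagara and updates the player-facing lifebar; FollowTrail is unused.
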(event `self.ReceiveBeginPlay`
  (`parent.ReceiveBeginPlay`)
  (bind _aswbp_lifebar (cast `/Game/UI/WBP_lifebar` (`WidgetComponent.GetWidget` (`self.Lifebar`))))
  (set `self.LifebarRef` _aswbp_lifebar)
  (bind _asbp_third_person_character (cast `/Game/ThirdPerson/Blueprints/BP_ThirdPersonCharacter` (`GameplayStatics.GetPlayerPawn` 0)))
  (set `self.Player` _asbp_third_person_character)
  (`KismetSystemLibrary.K2_SetTimerDelegate` (delegate `AttackPlayer`) 1.0 true))

(event `AttackPlayer`
  (bind _returnvalue (`self.K2_GetActorLocation`))
  (bind _returnvalue_2 (`self.K2_GetActorLocation`))
  (bind _returnvalue_3 (`self.K2_GetActorLocation`))
  (bind _returnvalue_4 (`self.K2_GetActorLocation` (`self.Player`)))
  (bind _returnvalue_5 (* (`self.GetActorForwardVector`) 300.0))
  (bind (_returnvalue_roll _returnvalue_pitch _returnvalue_yaw) (`KismetMathLibrary.BreakRotator` (`KismetMathLibrary.FindLookAtRotation` _returnvalue _returnvalue_4)))
  (if (`self.IsStunned`)
    _
    (elif (`self.InAttack`)
      _
      (elif (< (`KismetMathLibrary.Vector_Distance` _returnvalue_4 _returnvalue) 200.0)
        (set `self.InAttack` true)
        (`self.K2_SetActorRotation` (`KismetMathLibrary.MakeRotator` 0.0 0.0 _returnvalue_yaw))
        (`KismetSystemLibrary.DrawDebugArrow` _returnvalue_3 (+ _returnvalue_3 _returnvalue_5) 10.0 (struct :`R` 1.0 :`A` 1.0) 0.5 10.0)
        (`KismetSystemLibrary.Delay` 0.5)
        ;[1 1 1] Attack
        (bind _outhit (`KismetSystemLibrary.SphereTraceSingle` :`Start` _returnvalue_2 :`End` (+ _returnvalue_2 _returnvalue_5) :`Radius` 50.0 :`TraceChannel` "TraceTypeQuery3" :`DrawDebugType` "ForDuration"))
        (set `self.InAttack` false)
        (if (== (`.HitActor` (`GameplayStatics.BreakHitResult` _outhit)) (`self.Player`))
          (`self.Stunned` (`self.Player`) (`self.K2_GetActorLocation`)))))))

(event `self.ReceiveTick`
  (params (DeltaSeconds :type "Float (single-precision)"))
  (bind _lifebar (`self.Lifebar`))
  (bind _player (`self.Player`))
  (bind _niagara (`self.Niagara`))
  (if (not (or (`self.IsStaggered`) (`self.IsStunned`)))
    (`SceneComponent.SetVisibility` _niagara false false)
    (if (`self.InAttack`)
      _
      (elif (not (`/Game/ThirdPerson/Blueprints/BP_ThirdPersonCharacter.Is_Stunned` _player))
        (`parent.ReceiveTick` DeltaSeconds)
        (elif (<= (`self.GetDistanceTo` _player self) 1000.0)
          _
          (else
            _))))
    (else
      (`SceneComponent.SetVisibility` _niagara true false)))
  (set `/Game/UI/WBP_lifebar.CurrentHP` (`self.HitBar`) (`self.LifebarRef`))
  (`SceneComponent.K2_SetWorldRotation` _lifebar (`KismetMathLibrary.FindLookAtRotation` (`SceneComponent.K2_GetComponentLocation` _lifebar) (`self.K2_GetActorLocation` (`GameplayStatics.GetPlayerPawn` 0))) false false))

(event `/Game/Interface/BPI_StrikeInteraction.GetHit`
  (params (Hitcoordinate :type "Vector Structure") (ForwardVector :type "Vector Structure"))
  (bind _regenerationdelay (`self.RegenerationDelay`))
  (bind _hitbar (`self.HitBar`))
  (`self.Staggered`)
  (if (`self.IsStunned`)
    (`self.K2_AddActorWorldOffset` (0.0 0.0 100.0))
    (`self.LaunchCharacter` (+ (* ForwardVector 700.0) (0.0 0.0 100.0)))
    (else
      (`/Engine/EditorBlueprintResources/StandardMacros.DecrementInt` _hitbar
        (:`  `
          (if (<= _hitbar 0)
            (set `self.IsStunned` true)
            (set `self.HitBar` 0)
            (`KismetSystemLibrary.Delay` _regenerationdelay)
            (`/Engine/EditorBlueprintResources/StandardMacros.IncrementInt` (`self.HitBar`)
              (:`  `
                (`KismetSystemLibrary.Delay` _regenerationdelay)
                (`/Engine/EditorBlueprintResources/StandardMacros.IncrementInt` (`self.HitBar`)
                  (:`  `
                    (`KismetSystemLibrary.Delay` _regenerationdelay)
                    (`/Engine/EditorBlueprintResources/StandardMacros.IncrementInt` (`self.HitBar`)
                      (:`  `
                        (set `self.IsStunned` false)))))))))))))

(event `self.Stunned`
  (params (HitDirection :type "Vector Structure"))
  (set `self.IsStunned` true)
  (`KismetSystemLibrary.Delay` 1.0)
  (`self.K2_DestroyActor`))

(event `self.EatingRange.OnComponentBeginOverlap`
  (params (OverlappedComponent :type "PrimitiveComponent Object Reference") (OtherActor :type "Actor Object Reference") (OtherComp :type "PrimitiveComponent Object Reference") (OtherBodyIndex :type Integer) (bFromSweep :type Boolean) (SweepResult :type "HitResult Structure (by ref)"))
  (bind _target (`self.Target`))
  (bind _eatingrange (`self.EatingRange`))
  ;[1 0 0 1 64] Eating... deactivate
  (if (== OtherComp (`Actor.RootComponent` OtherActor))
    (if (== (`GameplayStatics.GetObjectClass` OtherActor) "/Game/Creatures/BP_CreatureHerd.BP_CreatureHerd_C")
      (bind _asbp_creature_herd (cast `/Game/Creatures/BP_CreatureHerd` OtherActor))
      (`/Engine/EditorBlueprintResources/StandardMacros.DoOnce` false :!label _label
        (:`Completed`
          (set `/Game/Creatures/BP_CreatureHerd.Grabbed` true _asbp_creature_herd)
          (set `self.InAttack` true)
          (set `self.Target` _asbp_creature_herd)
          (bind (_direction _lift) (`Timeline|EatCreature` :!via `PlayFromStart` :!label _label_2)
            (:`Update`
              (`self.K2_SetActorLocation` _target (`KismetMathLibrary.VLerp` (`self.K2_GetActorLocation` _target) (+ (`SceneComponent.K2_GetComponentLocation` (`self.CapsuleComponent`)) (0.0 0.0 150.0)) _lift) false false))
            (:`Finished`
              ;;[1 1 1] EatCreature - Faire un event pour ça
              (`self.K2_DestroyActor` (`self.Target`))
              (`KismetSystemLibrary.Delay` 5.0)
              (set `self.Target` null)
              (`|ExecutionSequence`
                (:`then_0`
                  (goto _label :!via `Reset`))
                (:`then_1`
                  (`PrimitiveComponent.SetCollisionEnabled` _eatingrange "NoCollision")
                  (`KismetSystemLibrary.Delay` 0.1)
                  (`PrimitiveComponent.SetCollisionEnabled` _eatingrange "QueryOnly")
                  (set `self.InAttack` false))))))))))

(event `self.Staggered`
  (bind _target (`self.Target`))
  (bind _charactermovement (`self.CharacterMovement`))
  (`|ExecutionSequence`
    (:`then_0`
      (goto _label_2 :!via `Stop`))
    (:`then_1`
      (set `self.IsStaggered` true)
      (`KismetSystemLibrary.Delay` 0.2)
      (set `self.IsStaggered` false)
      (`KismetSystemLibrary.Delay` 1.0)
      (goto _label :!via `Reset`))
    (:`then_2`
      (`/Engine/EditorBlueprintResources/StandardMacros.IsValid` _target
        (:`Is Valid`
          (`self.LaunchCharacter` _target (0.0 0.0 100.0) false true)
          (set `/Game/Creatures/BP_CreatureHerd.Grabbed` false _target))))
    (:`then_3`
      (set `CharacterMovementComponent.MaxWalkSpeed` 50.0 _charactermovement)
      (`KismetSystemLibrary.Delay` 1.0)
      (set `CharacterMovementComponent.MaxWalkSpeed` 500.0 _charactermovement))))

(fn `UserConstructionScript`
  (`parent.UserConstructionScript`))