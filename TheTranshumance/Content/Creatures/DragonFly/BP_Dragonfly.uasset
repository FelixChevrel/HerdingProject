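; Companion dragonfly that follows the player and carries out pull orders on a list of targets.
; Tick switches on CurrentOrder: Wait flies it to the player's DragonflyAttach point and snaps it there, while Pull flies it to each target in turn.
; DoOnce gates fire once per arrival; Push applies a large impulse opposite its forward vector to physics-simulating targets.
; After the last target it clears the list and returns to Wait.
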(event `self.ReceiveBeginPlay`
  (bind _asbp_third_person_character (cast `/Game/ThirdPerson/Blueprints/BP_ThirdPersonCharacter` (`GameplayStatics.GetPlayerPawn` 0)))
  (bind _output_get (set `self.Player` _asbp_third_person_character))
  (set `self.AttachPoint` (`/Game/ThirdPerson/Blueprints/BP_ThirdPersonCharacter.DragonflyAttach` _output_get)))

(event `self.ReceiveTick`
  (params (DeltaSeconds :type "Float (single-precision)"))
  (bind (_direction _distance) (`self.GetDirectionTarget`))
  (bind (_direction_2 _distance_2) (`self.GetDirectionPlayer`))
  (bind _target (`self.Target`))
  (bind _targetindexvalue (`self.TargetIndexValue`))
  (bind _attachpoint (`self.AttachPoint`))
  (switch `/Game/Creatures/DragonFly/ENUM_DragonflyOrders` (`self.CurrentOrder`)
    (:`NewEnumerator3`
      ;[1 1 1] Move To the player
      (if (not (< _distance_2 200.0))
        (`PawnMovementComponent.AddInputVector` (`self.FloatingPawnMovement`) _direction_2 false)
        (`self.TurnTowardMovement` _direction_2)
        (goto _label :!via `Reset`)
        (else
          (`|ExecutionSequence`
            (:`then_0`
              (`/Engine/EditorBlueprintResources/StandardMacros.DoOnce` false :!label _label
                (:`Completed`
                  (`self.K2_AttachToComponent` _attachpoint "None" "SnapToTarget" "SnapToTarget" "KeepWorld")
                  (`NavMovementComponent.StopActiveMovement` (`self.FloatingPawnMovement`)))))
            (:`then_1`
              (`SceneComponent.K2_SetWorldLocation` (`self.DefaultSceneRoot`) (`SceneComponent.K2_GetComponentLocation` _attachpoint) false false))))))
    (:`NewEnumerator0`
      (if (not (< _distance 200.0))
        (`PawnMovementComponent.AddInputVector` (`self.FloatingPawnMovement`) _direction false)
        (`self.TurnTowardMovement` _direction)
        (goto _label_2 :!via `Reset`)
        (else
          (`/Engine/EditorBlueprintResources/StandardMacros.DoOnce` false :!label _label_2
            (:`Completed`
              (`self.Push` (`|GetArrayItem` _target _targetindexvalue))
              (if (< _targetindexvalue (- (`KismetArrayLibrary.Array_Length` _target) 1))
                (`/Engine/EditorBlueprintResources/StandardMacros.IncrementInt` (`self.TargetIndexValue`))
                (else
                  (set `self.CurrentOrder` "NewEnumerator3")
                  (set `self.Target` (`|MakeArray`)))))))))))

(event `Push`
  (params (Component :type "PrimitiveComponent Object Reference"))
  (bind _asprimitive_component (cast `PrimitiveComponent` (`Actor.RootComponent` (`ActorComponent.GetOwner` Component))))
  (if (`SceneComponent.IsSimulatingPhysics` _asprimitive_component "None")
    (`PrimitiveComponent.AddImpulseAtLocation` _asprimitive_component (* (`self.GetActorForwardVector`) -100000.0) (`self.TargetPoint`) "None")
    (`KismetSystemLibrary.PrintString` "Success")))

(fn `GetDirectionPlayer`
  (returns (Direction :type "Vector Structure") (Distance :type "Float (double-precision)"))
  (bind _returnvalue (- (`SceneComponent.K2_GetComponentLocation` (`self.AttachPoint`)) (`self.K2_GetActorLocation`)))
  (return (`KismetMathLibrary.Normal` _returnvalue) (`KismetMathLibrary.VSize` _returnvalue)))

(fn `GetDirectionTarget`
  (returns (Direction :type "Vector Structure") (Distance :type "Float (double-precision)"))
  (bind _target (`self.Target`))
  (bind _returnvalue (- (`SceneComponent.K2_GetComponentLocation` (`|GetArrayItem` _target (`self.TargetIndexValue`))) (`self.K2_GetActorLocation`)))
  (if (> (`KismetArrayLibrary.Array_Length` _target) 0)
    (return (`KismetMathLibrary.Normal` _returnvalue) (`KismetMathLibrary.VSize` _returnvalue))
    (else
      (return (0.0 0.0 0.0) 0.0))))

(fn `TurnTowardMovement`
  (params (A :type "Vector Structure"))
  (bind _returnvalue (`self.K2_GetActorLocation`))
  (`self.K2_SetActorRotation` (`KismetMathLibrary.FindLookAtRotation` _returnvalue (+ A _returnvalue))))

(fn `UserConstructionScript`)