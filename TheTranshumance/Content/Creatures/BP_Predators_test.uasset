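; Predator creature Character with a hit-point lifebar that can be knocked into a stunned state.
; Hits drain HitBar until stun, which skips parent Tick, shows Niagara and makes further hits launch it.
; HitBar then regains three points on timed delays, though IsStunned is never cleared here; a separate Stunned event destroys the actor after a delay.
; Tick feeds HitBar to the lifebar widget and turns it toward the player.
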(event `self.ReceiveBeginPlay`
  (`parent.ReceiveBeginPlay`)
  (bind _aswbp_lifebar (cast `/Game/UI/WBP_lifebar` (`WidgetComponent.GetWidget` (`self.Lifebar`))))
  (set `self.LifebarRef` _aswbp_lifebar))

(event `self.ReceiveTick`
  (params (DeltaSeconds :type "Float (single-precision)"))
  (bind _lifebar (`self.Lifebar`))
  (if (not (`self.IsStunned`))
    (`parent.ReceiveTick` DeltaSeconds)
    (else
      (`SceneComponent.SetVisibility` (`self.Niagara`) true false)))
  (set `/Game/UI/WBP_lifebar.CurrentHP` (`self.HitBar`) (`self.LifebarRef`))
  (`SceneComponent.K2_SetWorldRotation` _lifebar (`KismetMathLibrary.FindLookAtRotation` (`SceneComponent.K2_GetComponentLocation` _lifebar) (`self.K2_GetActorLocation` (`GameplayStatics.GetPlayerPawn` 0))) false false))

(event `/Game/GPE/BPI_StrikeInteraction.GetHit`
  (params (Hitcoordinate :type "Vector Structure") (ForwardVector :type "Vector Structure"))
  (bind _regenerationdelay (`self.RegenerationDelay`))
  (bind _hitbar (`self.HitBar`))
  (if (`self.IsStunned`)
    (`self.LaunchCharacter` (+ (* ForwardVector 500.0) (0.0 0.0 100.0)))
    (else
      (`/Engine/EditorBlueprintResources/StandardMacros.DecrementInt` _hitbar
        (:`  `
          (if (<= _hitbar 0)
            (set `self.IsStunned` true)
            (set `self.HitBar` 0)
            (`KismetSystemLibrary.Delay` _regenerationdelay)
            (`/Engine/EditorBlueprintResources/StandardMacros.IncrementInt` (`self.HitBar`)
              (:`  `
                (`KismetSystemLibrary.Delay` _regenerationdelay)
                (`/Engine/EditorBlueprintResources/StandardMacros.IncrementInt` (`self.HitBar`)
                  (:`  `
                    (`KismetSystemLibrary.Delay` _regenerationdelay)
                    (`/Engine/EditorBlueprintResources/StandardMacros.IncrementInt` (`self.HitBar`))))))))))))

(event `/Game/Interface/BPI_Stunnable.Stunned`
  (params (HitDirection :type "Vector Structure"))
  (set `self.IsStunned` true)
  (`KismetSystemLibrary.Delay` 1.0)
  (`self.K2_DestroyActor`))

(fn `UserConstructionScript`
  (`parent.UserConstructionScript`))