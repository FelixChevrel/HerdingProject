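; BP_CreatureHerd is a creature Character that herds by keeping per-class preferred distances from nearby actors.
; DetectionRange overlaps maintain the actor list, which a start-staggered timer turns into a MovementGoal by summing clamped, weighted attraction or repulsion, with some classes repel-only.
; Tick feeds that goal plus periodic random skitter into movement unless the creature is grabbed.
; Events also handle delayed bounces, launches toward the player and freezing in sap.
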(event `GetDirection`
  (bind _acceptancerange (`self.AcceptanceRange`))
  ;[1 1 1] Get CurrentVector
  (set `self.MovementGoal` (0.0 0.0 0.0))
  (for _array_element (`self.ActorsList`)
    (bind _returnvalue (`GameplayStatics.GetObjectClass` _array_element))
    (bind (_value _returnvalue_2) (`BlueprintMapLibrary.Map_Find` (`self.DistanceFavorableArray`) _returnvalue))
    (if _returnvalue_2
      (bind _returnvalue_3 (- (`self.K2_GetActorLocation` _array_element) (`self.K2_GetActorLocation`)))
      (set `self.MovementGoal` (+ (`self.MovementGoal`) (* (`KismetMathLibrary.Normal` _returnvalue_3) (* (/ (`KismetMathLibrary.FClamp` (- (`KismetMathLibrary.VSize` _returnvalue_3) _value) (* _acceptancerange -1.0) (`KismetMathLibrary.SelectFloat` _acceptancerange 0.0 (`BlueprintMapLibrary.Map_Find` (`self.MinDistanceDict`) _returnvalue))) (`self.AcceptanceRange`)) (`BlueprintMapLibrary.Map_Find` (`self.HerdingInstinctMult`) _returnvalue)))))))
  (set `self.MovementGoal` (`self.MovementGoal`)))

(event `self.ReceiveBeginPlay`
  (bind _returnvalue (/ (`KismetMathLibrary.Conv_IntToDouble` (`KismetMathLibrary.RandomInteger` 10)) 100.0))
  (`KismetSystemLibrary.K2_SetTimerDelegate` (delegate `SetRandomSkitter`) 2.0 true)
  (`KismetSystemLibrary.PrintString` (`KismetStringLibrary.Conv_DoubleToString` _returnvalue))
  (`KismetSystemLibrary.Delay` _returnvalue)
  (`KismetSystemLibrary.K2_SetTimerDelegate` (delegate `GetDirection`) 0.1 true))

(event `SetRandomSkitter`
  (set `self.RandomVector` (`KismetMathLibrary.MakeVector` (`KismetMathLibrary.RandomFloatInRange` -0.25 0.25) (`KismetMathLibrary.RandomFloatInRange` -0.25 0.25)))
  (`KismetSystemLibrary.Delay` 1.0))

(event `self.ReceiveTick`
  (params (DeltaSeconds :type "Float (single-precision)"))
  (if (not (`self.Grabbed`))
    (`PawnMovementComponent.AddInputVector` (`self.CharacterMovement`) (+ (`self.MovementGoal`) (`self.RandomVector`)) false)))

(event `self.DetectionRange.OnComponentBeginOverlap`
  (params (OverlappedComponent :type "PrimitiveComponent Object Reference") (OtherActor :type "Actor Object Reference") (OtherComp :type "PrimitiveComponent Object Reference") (OtherBodyIndex :type Integer) (bFromSweep :type Boolean) (SweepResult :type "HitResult Structure (by ref)"))
  (if (== OtherComp (`Actor.RootComponent` OtherActor))
    (`KismetArrayLibrary.Array_AddUnique` (`self.ActorsList`) OtherActor)))

(event `self.DetectionRange.OnComponentEndOverlap`
  (params (OverlappedComponent :type "PrimitiveComponent Object Reference") (OtherActor :type "Actor Object Reference") (OtherComp :type "PrimitiveComponent Object Reference") (OtherBodyIndex :type Integer))
  (if (== OtherComp (`Actor.RootComponent` OtherActor))
    (`KismetArrayLibrary.Array_RemoveItem` (`self.ActorsList`) OtherActor)))

(event `/Game/Interface/BPI_EnvironmentInteraction.BOUNCE`
  (params (Delay :type "Float (double-precision)") (Direction :type "Vector Structure") (Power :type "Float (double-precision)"))
  (`/Engine/EditorBlueprintResources/StandardMacros.DoOnce` false :!label _label
    (:`Completed`
      (`KismetSystemLibrary.Delay` Delay)
      (`self.LaunchCharacter` (* Direction Power) false true)
      (goto _label :!via `Reset`))))

(event `/Game/Interface/BPI_DragonflyInteraction.PushTowardPlayer`
  (`self.LaunchCharacter` (* (+ (`KismetMathLibrary.Normal` (- (`self.K2_GetActorLocation` (`GameplayStatics.GetPlayerPawn` 0)) (`self.K2_GetActorLocation`))) (0.0 0.0 1.0)) 500.0) true true))

(event `/Game/Interface/BPI_EnvironmentInteraction.STUCK`
  (params (OnOrOff :type Boolean))
  (bind _charactermovement (`self.CharacterMovement`))
  (if OnOrOff
    (set `CharacterMovementComponent.MaxWalkSpeed` 0.0 _charactermovement)
    (set `CharacterMovementComponent.GravityScale` 0.0 _charactermovement)
    (set `MovementComponent.Velocity` (0.0 0.0 0.0) _charactermovement)
    (set `self.InSap` true)
    (else
      (set `CharacterMovementComponent.MaxWalkSpeed` 400.0 _charactermovement)
      (set `CharacterMovementComponent.GravityScale` 1.0 _charactermovement)
      (set `self.InSap` false))))

(fn `UserConstructionScript`)