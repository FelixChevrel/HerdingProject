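; BP_Water_Despawner is a water hazard that returns the player to safe ground and destroys other characters that fall in.
; A looping timer records the player's location whenever they are walking on the ground.
; When the player overlaps the box and passes CheckValidity, they teleport slightly above that saved spot, lose their velocity and get stunned.
; Otherwise, any Character whose root component overlaps is destroyed.
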(event `self.ReceiveBeginPlay`
  (`KismetSystemLibrary.K2_SetTimerDelegate` (delegate `CheckPlayerLocation`) 1.0 true)
  (bind _asbp_third_person_character (cast `/Game/ThirdPerson/Blueprints/BP_ThirdPersonCharacter` (`GameplayStatics.GetPlayerPawn` 0)))
  (set `self.Player` _asbp_third_person_character))

(event `CheckPlayerLocation`
  (bind _player (`self.Player`))
  (if (`NavMovementComponent.IsMovingOnGround` (`Character.CharacterMovement` _player))
    (set `self.PlayerLastOnGround` (`self.K2_GetActorLocation` _player))))

(event `self.Box.OnComponentBeginOverlap`
  (params (OverlappedComponent :type "PrimitiveComponent Object Reference") (OtherActor :type "Actor Object Reference") (OtherComp :type "PrimitiveComponent Object Reference") (OtherBodyIndex :type Integer) (bFromSweep :type Boolean) (SweepResult :type "HitResult Structure (by ref)"))
  (bind _player (`self.Player`))
  (bind _playerlastonground (`self.PlayerLastOnGround`))
  (if (`/Game/Interface/MacroLib_GeneralUtility.CheckValidity` OtherActor (`self.Player`) OtherComp)
    ;[1 1 1] Teleport
    (`self.K2_SetActorLocation` _player (+ _playerlastonground (0.0 0.0 100.0)) false false)
    (set `MovementComponent.Velocity` (0.0 0.0 0.0) (`Character.CharacterMovement` _player))
    (`/Game/Interface/BPI_Stunnable.Stunned` _player _playerlastonground)
    (elif (and (`KismetMathLibrary.ClassIsChildOf` (`GameplayStatics.GetObjectClass` OtherActor) "/Script/Engine.Character") (== OtherComp (`Actor.RootComponent` OtherActor)))
      (`self.K2_DestroyActor` OtherActor))))

(fn `UserConstructionScript`)