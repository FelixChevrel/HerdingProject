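; Flying pet dragonfly that follows the player, waits at a spot, or goes to a target to interact or fetch it.
; A looping timer re-issues AI moves for the current order, mostly without pathfinding.
; On overlapping its target, it uses BPI_PetInteractible, where only Cut triggers a reaction, or attaches non-interface targets as cargo.
; It then resumes following, dropping cargo near the player and restoring any disabled physics.
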(event `self.ReceiveBeginPlay`
  (`KismetSystemLibrary.K2_SetTimerDelegate` (delegate `GoToPlayer`) 0.2 true)
  (`CharacterMovementComponent.SetMovementMode` (`self.CharacterMovement`) "MOVE_Flying" 0))

(event `GoToPlayer`
  (bind _target (`self.target`))
  (bind _cargo (`self.Cargo`))
  (switch `petOrder` (`self.currentOrder`)
    (:`follow`
      (`AIController.MoveToLocation` (`AIBlueprintHelperLibrary.GetAIController` self) (+ (`self.K2_GetActorLocation` (`GameplayStatics.GetPlayerPawn` 0)) (0.0 0.0 80.0)) 1.0 true false false true null true)
      (if (< (`self.GetDistanceTo` (`GameplayStatics.GetPlayerPawn` 0) self) 200.0)
        (if (`self.Holding`)
          (`KismetSystemLibrary.PrintString` "release")
          (`self.K2_DetachFromActor` _cargo "KeepWorld" "KeepWorld" "KeepWorld")
          (`self.SetActorEnableCollision` _cargo true)
          (set `self.Holding` false)
          (if (`self.WasPhysic`)
            (bind _asprimitive_component (cast `PrimitiveComponent` (`Actor.RootComponent` (`self.Cargo`))))
            (`PrimitiveComponent.SetSimulatePhysics` _asprimitive_component true))
          (set `self.Cargo` null)
          (set `self.WasPhysic` false))))
    (:`wait`
      (`AIController.MoveToLocation` (`AIBlueprintHelperLibrary.GetAIController` self) (`self.WaitSpot`) 10.0 true true false true null true))
    (:`interact`
      (`/Engine/EditorBlueprintResources/StandardMacros.IsValid` _target
        (:`Is Valid`
          (if (`KismetSystemLibrary.DoesImplementInterface` _target "/Game/GAMEPLAY/INTERFACE/BPI_PetInteractible.BPI_PetInteractible_C")
            (if (not (`self.Holding`))
              (bind (_specificspot _coordinates) (message `/Game/GAMEPLAY/INTERFACE/BPI_PetInteractible.Where?` _target))
              (if _specificspot
                (`AIController.MoveToLocation` (`AIBlueprintHelperLibrary.GetAIController` self) _coordinates 10.0 true false false true null true)
                (`KismetSystemLibrary.PrintString` (`KismetStringLibrary.Conv_VectorToString` _coordinates))
                (else
                  (`AIController.MoveToActor` (`AIBlueprintHelperLibrary.GetAIController` self) _target 10.0 true false true null true :!label _label))))
            (else
              (goto _label))))))))

(event `self.takeAction`
  (bind _target (`self.target`))
  (bind _rootcomponent (`Actor.RootComponent` (`self.target`)))
  (if (`KismetSystemLibrary.DoesImplementInterface` (`self.target`) "/Game/GAMEPLAY/INTERFACE/BPI_PetInteractible.BPI_PetInteractible_C")
    (bind _orders (message `/Game/GAMEPLAY/INTERFACE/BPI_PetInteractible.WhatType?` (`self.target`)))
    (switch `actionTypes` _orders
      (:`dragCut`
        (`KismetSystemLibrary.PrintString` "Cut")
        (message `/Game/GAMEPLAY/INTERFACE/BPI_PetInteractible.Reaction` (`self.target`)))
      (:`dragBring`
        (`KismetSystemLibrary.PrintString` "Bring"))
      (:`dragStun`
        (`KismetSystemLibrary.PrintString` "Stun")))
    (set `self.target` null)
    (set `self.InOrder` false)
    (set `self.Holding` false)
    (set `self.currentOrder` "follow")
    (else
      (if (not (`self.Holding`))
        (if (`SceneComponent.IsSimulatingPhysics` _rootcomponent "None")
          (bind _asprimitive_component (cast `PrimitiveComponent` _rootcomponent))
          (`PrimitiveComponent.SetSimulatePhysics` _asprimitive_component false)
          (`KismetSystemLibrary.PrintString` "Break Physic")
          (set `self.WasPhysic` true)
          (else
            (set `self.WasPhysic` false)))
        (`self.K2_AttachToComponent` _target (`self.AttachPoint`) "None" "SnapToTarget" "KeepWorld" "KeepWorld" false)
        (bind _output_get (set `self.Cargo` _target))
        (`self.SetActorEnableCollision` _output_get false)
        (set `self.Holding` true))
      (set `self.target` null)
      (set `self.InOrder` false)
      (set `self.currentOrder` "follow"))))

(event `self.CancelOrder`
  (set `self.currentOrder` "follow")
  (set `self.target` null)
  (`|ExecutionSequence`))

(event `self.drop`)

(event `self.Sphere4.OnComponentBeginOverlap`
  (params (OverlappedComponent :type "PrimitiveComponent Object Reference") (OtherActor :type "Actor Object Reference") (OtherComp :type "PrimitiveComponent Object Reference") (OtherBodyIndex :type Integer) (bFromSweep :type Boolean) (SweepResult :type "HitResult Structure (by ref)"))
  (bind _target (`self.target`))
  (`/Engine/EditorBlueprintResources/StandardMacros.IsValid` _target
    (:`Is Valid`
      (if (== OtherActor _target)
        (`self.takeAction`)
        (`KismetSystemLibrary.PrintString` "GetTarget")))))

(fn `UserConstructionScript`)