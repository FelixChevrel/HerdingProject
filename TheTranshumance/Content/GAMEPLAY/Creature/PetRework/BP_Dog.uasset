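; Dog pet character that follows the player, waits at a spot, or interacts with a target, and can be thrown.
; A one-second timer re-issues AI moves for the current order.
; Overlapping the target triggers dig, pull or attack, chosen through BPI_PetInteractible messages.
; Timelines scale dig piles, drag dog and target backward unless a sphere trace blocks, and repeat attacks while target feedback stays positive.
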(event `self.ReceiveBeginPlay`
  (`KismetSystemLibrary.K2_SetTimerDelegate` (delegate `GoTooPlayer`) 1.0 true))

(event `GoTooPlayer`
  (bind _target (`self.target`))
  (switch `petOrder` (`self.currentOrder`)
    (:`follow`
      (`AIController.MoveToActor` (`AIBlueprintHelperLibrary.GetAIController` self) (`GameplayStatics.GetPlayerPawn` 0) 100.0 true true true null true))
    (:`wait`
      (`AIController.MoveToLocation` (`AIBlueprintHelperLibrary.GetAIController` self) (`self.WaitSpot`) 10.0 true true false true null true))
    (:`interact`
      (`/Engine/EditorBlueprintResources/StandardMacros.IsValid` _target
        (:`Is Valid`
          (if (not (`self.Locked`))
            (bind (_specificspot _coordinates) (message `/Game/GAMEPLAY/INTERFACE/BPI_PetInteractible.Where?` _target))
            (if _specificspot
              (`AIController.MoveToLocation` (`AIBlueprintHelperLibrary.GetAIController` self) _coordinates 10.0 true true false true null true)
              (else
                (`AIController.MoveToActor` (`AIBlueprintHelperLibrary.GetAIController` self) _target 30.0 true true true null true)))))))))

(event `self.takeAction`
  (bind _target (`self.target`))
  (bind _target_2 (`self.target`))
  (bind _returnvalue (+ (`self.K2_GetActorLocation`) (0.0 0.0 25.0)))
  (if (`KismetSystemLibrary.DoesImplementInterface` (`self.target`) "/Game/GAMEPLAY/INTERFACE/BPI_PetInteractible.BPI_PetInteractible_C")
    (bind _orders (message `/Game/GAMEPLAY/INTERFACE/BPI_PetInteractible.WhatType?` (`self.target`)))
    (switch `actionTypes` _orders
      (:`dogDig`
        (set `self.PileScale` (`self.GetActorScale3D` _target))
        (bind (_direction _newtrack_0) (`Timeline|DigMedium` :!via `PlayFromStart` :!label _label)
          (:`Update`
            (`self.SetActorScale3D` _target (* _newtrack_0 (`self.PileScale`))))
          (:`Finished`
            (message `/Game/GAMEPLAY/INTERFACE/BPI_PetInteractible.Reaction` _target)
            (set `self.target` null :!label _label_2)
            (set `self.InOrder` false)
            (set `self.Locked` false)
            (set `self.currentOrder` "follow"))))
      (:`dogPull`
        (`Controller.StopMovement` (`AIBlueprintHelperLibrary.GetAIController` self))
        (set `self.Locked` true)
        (bind (_specificspot _coordinates _specificrot _rot) (message `/Game/GAMEPLAY/INTERFACE/BPI_PetInteractible.Where?` (`self.target`)))
        (`self.K2_SetActorRotation` self _rot false)
        (`self.K2_SetActorLocation` self _coordinates false false)
        (bind (_direction_2 _newtrack_0_2) (`Timeline|PullTimeline` :!via `PlayFromStart`)
          (:`Update`
            (bind _returnvalue_2 (* (* (`self.GetActorForwardVector` self) -1.0) (* _newtrack_0_2 3.0)))
            (bind (_outhit _returnvalue_3) (`KismetSystemLibrary.SphereTraceSingle` _returnvalue (+ _returnvalue _returnvalue_2) 0.0 "TraceTypeQuery1"))
            (if (not _returnvalue_3)
              (`self.K2_AddActorWorldOffset` self _returnvalue_2 false false)
              (`self.K2_AddActorWorldOffset` (`self.target`) _returnvalue_2 false false)))
          (:`Finished`
            (goto _label_2))))
      (:`dogAttack`
        (`KismetSystemLibrary.PrintString` "Attack")
        (`Timeline|AttakLoop` :!via `PlayFromStart` :!label _label_3
          (:`Finished`
            (if (< (`self.GetDistanceTo` _target_2 self) 50.0)
              (message `/Game/GAMEPLAY/INTERFACE/BPI_PetInteractible.Attack` _target_2 (`self.K2_GetActorLocation`) (`self.GetActorForwardVector`) 1000.0))
            (bind _hpleft (message `/Game/GAMEPLAY/INTERFACE/BPI_PetInteractible.AttackFeedbackData` _target_2))
            (if (> _hpleft 0)
              (goto _label_3 :!via `PlayFromStart`)
              (else
                (goto _label_2)))))))))

(event `self.CancelOrder`
  (set `self.currentOrder` "follow")
  (set `self.target` null)
  (`|ExecutionSequence`
    (:`then_0`
      (goto _label :!via `Stop`))
    (:`then_1`
      (goto _label_3 :!via `Stop`))))

(event `self.drop`)

(event `self.Sphere4.OnComponentBeginOverlap`
  (params (OverlappedComponent :type "PrimitiveComponent Object Reference") (OtherActor :type "Actor Object Reference") (OtherComp :type "PrimitiveComponent Object Reference") (OtherBodyIndex :type Integer) (bFromSweep :type Boolean) (SweepResult :type "HitResult Structure (by ref)"))
  (bind _target (`self.target`))
  (`/Engine/EditorBlueprintResources/StandardMacros.IsValid` _target
    (:`Is Valid`
      (if (== OtherActor _target)
        (`self.takeAction`)))))

(event `/Game/GAMEPLAY/INTERFACE/BPI_EnvironmentInteraction.GetThrown`
  (params (Impulse :type "Vector Structure"))
  (`self.LaunchCharacter` Impulse true true))

(fn `GetWeight`
  (returns (Weight :type Integer))
  (return 0))

(fn `UserConstructionScript`)