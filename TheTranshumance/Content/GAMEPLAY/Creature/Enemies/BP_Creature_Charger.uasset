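; Charger enemy creature that periodically checks whether the player is in range, then turns toward them and rushes in a straight line.
; A timeline drives swept movement along ChargeArrow, throwing the player or environment-interaction actors it hits.
; Hitting the player ends the charge with only a debug damage print, while other obstacles briefly stun it.
; Parent tick pauses during charge or stun, and incoming damage is rate-limited, updating the health bar.
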(event `CanAttack`
  (bind (_returnvalue_roll _returnvalue_pitch _returnvalue_yaw) (`KismetMathLibrary.BreakRotator` (`KismetMathLibrary.FindLookAtRotation` (`self.K2_GetActorLocation`) (`self.K2_GetActorLocation` (`GameplayStatics.GetPlayerPawn` 0)))))
  (bind _returnvalue (* (+ (* (`SceneComponent.GetForwardVector` (`self.ChargeArrow`)) -1.0) (0.0 0.0 2.0)) 300.0))
  (if (not (`self.Charging`))
    ;[1 1 1] Check if the conditionas are ok :
    (if (< (`self.GetDistanceTo` (`GameplayStatics.GetPlayerPawn` 0) self) (`self.AttackRange`))
      (set `self.Charging` true)
      ;[1 1 1] Set rotation
      (`self.K2_SetActorRotation` (`KismetMathLibrary.MakeRotator` 0.0 0.0 _returnvalue_yaw))
      ;[1 1 1] Play animation of charge
      (bind (_direction _chargespeed) (`Timeline|Charge` :!via `PlayFromStart` :!label _label)
        (:`Update`
          (bind _sweephitresult (`self.K2_AddActorWorldOffset` (* (`SceneComponent.GetForwardVector` (`self.ChargeArrow`)) _chargespeed (`self.chargeSpeed`)) true))
          (bind (_bblockinghit _binitialoverlap _time _distance _location _impactpoint _normal _impactnormal _physmat _hitactor) (`GameplayStatics.BreakHitResult` _sweephitresult))
          (if _bblockinghit
            (if (== _hitactor (`GameplayStatics.GetPlayerPawn` 0))
              (`KismetSystemLibrary.PrintString` "DAMAGES")
              (message `/Game/GAMEPLAY/INTERFACE/BPI_EnvironmentInteraction.GetThrown` _hitactor _returnvalue)
              (set `self.Charging` false :!label _label_2)
              (goto _label :!via `Stop`)
              (elif (`KismetSystemLibrary.DoesImplementInterface` _hitactor "/Game/GAMEPLAY/INTERFACE/BPI_EnvironmentInteraction.BPI_EnvironmentInteraction_C")
                (message `/Game/GAMEPLAY/INTERFACE/BPI_EnvironmentInteraction.GetThrown` _hitactor _returnvalue)
                (else
                  (`KismetSystemLibrary.PrintString` "Stop")
                  (`|ExecutionSequence`
                    (:`then_0`
                      (goto _label_2))
                    (:`then_1`
                      (set `self.Stuned` true)
                      (`KismetSystemLibrary.Delay` 1.0)
                      (set `self.Stuned` false))))))))
        (:`Finished`
          (set `self.Charging` false))))))

(event `self.ReceiveBeginPlay`
  (`parent.ReceiveBeginPlay`)
  (`KismetSystemLibrary.K2_SetTimerDelegate` (delegate `CanAttack`) 10.0 true) ; Every 5 seconds, check if the player is in range
  (bind _aswbp_lifebar (cast `/Game/UI/WBP_lifebar` (`WidgetComponent.GetWidget` (`self.Widget`))))
  (set `self.HP_bar` _aswbp_lifebar))

(event `self.ReceiveTick`
  (params (DeltaSeconds :type "Float (single-precision)"))
  (if (and (not (`self.Charging`)) (not (`self.Stuned`)))
    (`parent.ReceiveTick` DeltaSeconds)))

(event `/Game/GAMEPLAY/INTERFACE/BPI_PlayerInteractible.TakeDamages`
  (params (DamageTaken :type Integer))
  (`/Engine/EditorBlueprintResources/StandardMacros.DoOnce` false :!label _label_3
    (:`Completed`
      (bind _output_get (set `self.HP` (- (`self.HP`) 1)))
      (set `/Game/UI/WBP_lifebar.CurrentHP` _output_get (`self.HP_bar`))
      (if (< _output_get 1)
        (`self.K2_DestroyActor`)
        (else
          (`KismetSystemLibrary.Delay` 1.0)
          (goto _label_3 :!via `Reset`))))))

(fn `UserConstructionScript`
  (`parent.UserConstructionScript`))