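; Herd creature character that steers around nearby actors and can be marked into the player's CreatureHerd list.
; A looping timer, randomly offset at start, sums pulls and pushes from actors in DetectionRange, using per-class preferred distance and instinct weight maps.
; Tick feeds that flattened vector into movement unless grabbed and shows a cube while marked.
; BOUNCE launches it after a delay, STUCK freezes it in sap, and debug drawing visualizes herding ranges.
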(event `GetDirection`
  (bind _returnvalue (`self.K2_GetActorLocation`))
  (bind _acceptancerange (`self.AcceptanceRange`))
  (bind _acceptancerange_2 (`self.AcceptanceRange`))
  (set `self.MovementGoal` (0.0 0.0 0.0))
  (for _array_element (`self.ActorsList`)
    (if (not (== _array_element self))
      (bind _returnvalue_2 (`GameplayStatics.GetObjectClass` _array_element))
      (bind (_value _returnvalue_3) (`BlueprintMapLibrary.Map_Find` (`self.DistanceFavorableArray`) _returnvalue_2))
      (bind (_value_2 _returnvalue_4) (`BlueprintMapLibrary.Map_Find` (`self.MinDistanceDict`) _returnvalue_2))
      (bind (_value_3 _returnvalue_5) (`BlueprintMapLibrary.Map_Find` (`self.HerdingInstinctMult`) _returnvalue_2))
      (if (and _returnvalue_3 _returnvalue_4 _returnvalue_5)
        (`|ExecutionSequence`
          (:`then_0`
            (bind _returnvalue_6 (`self.K2_GetActorLocation` _array_element))
            (bind _returnvalue_7 (- _returnvalue_6 _returnvalue))
            (bind _returnvalue_8 (`KismetMathLibrary.FClamp` (- (`KismetMathLibrary.VSize` _returnvalue_7) _value) (* _acceptancerange -1.0) (`KismetMathLibrary.SelectFloat` _acceptancerange 0.0 _value_2)))
            (bind _returnvalue_9 (/ _returnvalue_8 (* _acceptancerange_2 2.0)))
            (`self.DebugHerdingBehavior` _returnvalue _returnvalue_6 _returnvalue_9 _returnvalue_9 _value))
          (:`then_1`
            (if (`.ReturnValue` (`BlueprintMapLibrary.Map_Find` (`self.HerdingForwardMult`) _returnvalue_2))
              _
              (else
                _))
            (set `self.MovementGoal` (+ (`self.MovementGoal`) (* (* (`KismetMathLibrary.Normal` _returnvalue_7) (/ _returnvalue_8 _acceptancerange_2)) _value_3)))))))))

(event `self.ReceiveBeginPlay`
  (`KismetSystemLibrary.K2_SetTimerDelegate` (delegate `SetRandomSkitter`) 2.0 true)
  (`KismetSystemLibrary.Delay` (/ (`KismetMathLibrary.Conv_IntToDouble` (`KismetMathLibrary.RandomInteger` 10)) 100.0))
  (`KismetSystemLibrary.K2_SetTimerDelegate` (delegate `GetDirection`) 0.1 true))

(event `SetRandomSkitter`)

(event `self.ReceiveTick`
  (params (DeltaSeconds :type "Float (single-precision)"))
  (`SceneComponent.SetVisibility` (`self.Cube`) (`self.Marked`) false)
  (if (not (`self.IsGrabbed`))
    (`PawnMovementComponent.AddInputVector` (`self.CharacterMovement`) (+ (`KismetMathLibrary.ProjectVectorOnToPlane` (`self.MovementGoal`) (0.0 0.0 1.0)) (`self.RandomVector`)) false)))

(event `self.DetectionRange.OnComponentBeginOverlap`
  (params (OverlappedComponent :type "PrimitiveComponent Object Reference") (OtherActor :type "Actor Object Reference") (OtherComp :type "PrimitiveComponent Object Reference") (OtherBodyIndex :type Integer) (bFromSweep :type Boolean) (SweepResult :type "HitResult Structure (by ref)"))
  (if (== OtherComp (`Actor.RootComponent` OtherActor))
    (`KismetArrayLibrary.Array_AddUnique` (`self.ActorsList`) OtherActor)))

(event `self.DetectionRange.OnComponentEndOverlap`
  (params (OverlappedComponent :type "PrimitiveComponent Object Reference") (OtherActor :type "Actor Object Reference") (OtherComp :type "PrimitiveComponent Object Reference") (OtherBodyIndex :type Integer))
  (if (== OtherComp (`Actor.RootComponent` OtherActor))
    (`KismetArrayLibrary.Array_RemoveItem` (`self.ActorsList`) OtherActor)))

(event `/Game/GAMEPLAY/INTERFACE/BPI_EnvironmentInteraction.BOUNCE`
  (params (Delay :type "Float (double-precision)") (Direction :type "Vector Structure") (Power :type "Float (double-precision)"))
  (`/Engine/EditorBlueprintResources/StandardMacros.DoOnce` false :!label _label
    (:`Completed`
      (`KismetSystemLibrary.Delay` Delay)
      (`self.LaunchCharacter` (* Direction Power) false true)
      (goto _label :!via `Reset`))))

(event `/Game/GAMEPLAY/INTERFACE/BPI_EnvironmentInteraction.STUCK`
  (params (OnOrOff :type Boolean))
  (bind _charactermovement (`self.CharacterMovement`))
  (if OnOrOff
    (set `CharacterMovementComponent.MaxWalkSpeed` 0.0 _charactermovement)
    (set `CharacterMovementComponent.GravityScale` 0.0 _charactermovement)
    (set `MovementComponent.Velocity` (0.0 0.0 0.0) _charactermovement)
    (set `self.InSap` true)
    (else
      (set `CharacterMovementComponent.MaxWalkSpeed` 400.0 _charactermovement)
      (set `CharacterMovementComponent.GravityScale` 1.0 _charactermovement)
      (set `self.InSap` false))))

(event `self.ReceiveDestroyed`
  (bind _asbp_third_person_character (cast `/Game/GAMEPLAY/PlayerCharacter/Blueprints/BP_ThirdPersonCharacter` (`GameplayStatics.GetPlayerPawn` 0)))
  (`KismetArrayLibrary.Array_RemoveItem` (`/Game/GAMEPLAY/PlayerCharacter/Blueprints/BP_ThirdPersonCharacter.CreatureHerd` _asbp_third_person_character) self))

(fn `GetWeight`
  (returns (Weight :type Integer))
  (return 1))

(fn `MarkHerd`
  (params (Player :type "/Game/GAMEPLAY/PlayerCharacter/Blueprints/BP_ThirdPersonCharacter Object Reference") (Unmark :type Boolean))
  (returns (IsHerd :type Boolean))
  (bind _creatureherd (`/Game/GAMEPLAY/PlayerCharacter/Blueprints/BP_ThirdPersonCharacter.CreatureHerd` Player))
  (bind _returnvalue (`KismetArrayLibrary.Array_Contains` _creatureherd self))
  (if Unmark
    (set `self.Marked` false)
    (if _returnvalue
      (`KismetArrayLibrary.Array_RemoveItem` _creatureherd self))
    (return false)
    (else
      (if (not _returnvalue)
        (`KismetArrayLibrary.Array_Add` _creatureherd self)
        (set `self.Marked` true))
      (return true))))

(fn `UserConstructionScript`)