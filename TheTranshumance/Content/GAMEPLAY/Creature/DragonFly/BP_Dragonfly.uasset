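; BP_Dragonfly is a dragonfly creature Blueprint that provides movement helpers for steering toward an attach point or a set of targets.
; BeginPlay caches the third-person player character and clears AttachPoint.
; GetDirectionPlayer and GetDirectionTarget return direction and distance to AttachPoint or the indexed Target, while TurnTowardMovement rotates the actor along a given vector.
; Tick and Push are empty, and nothing in these graphs calls the helpers or moves the actor.
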(event `Push`
  (params (Component :type "PrimitiveComponent Object Reference")))

(event `self.ReceiveBeginPlay`
  (bind _asbp_third_person_character (cast `/Game/GAMEPLAY/PlayerCharacter/Blueprints/BP_ThirdPersonCharacter` (`GameplayStatics.GetPlayerPawn` 0)))
  (set `self.Player` _asbp_third_person_character)
  (set `self.AttachPoint` null))

(event `self.ReceiveTick`
  (params (DeltaSeconds :type "Float (single-precision)")))

(fn `GetDirectionPlayer`
  (returns (Direction :type "Vector Structure") (Distance :type "Float (double-precision)"))
  (bind _returnvalue (- (`SceneComponent.K2_GetComponentLocation` (`self.AttachPoint`)) (`self.K2_GetActorLocation`)))
  (return (`KismetMathLibrary.Normal` _returnvalue) (`KismetMathLibrary.VSize` _returnvalue)))

(fn `GetDirectionTarget`
  (returns (Direction :type "Vector Structure") (Distance :type "Float (double-precision)"))
  (bind _target (`self.Target`))
  (bind _returnvalue (- (`SceneComponent.K2_GetComponentLocation` (`|GetArrayItem` _target (`self.TargetIndexValue`))) (`self.K2_GetActorLocation`)))
  (if (> (`KismetArrayLibrary.Array_Length` _target) 0)
    (return (`KismetMathLibrary.Normal` _returnvalue) (`KismetMathLibrary.VSize` _returnvalue))
    (else
      (return (0.0 0.0 0.0) 0.0))))

(fn `TurnTowardMovement`
  (params (A :type "Vector Structure"))
  (bind _returnvalue (`self.K2_GetActorLocation`))
  (`self.K2_SetActorRotation` (`KismetMathLibrary.FindLookAtRotation` _returnvalue (+ A _returnvalue))))

(fn `UserConstructionScript`)