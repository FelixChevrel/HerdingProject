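; BP_HerdManager tracks herd creature deaths and pen counts, and unlocks progress objects as gathered totals reach set milestones.
; On BeginPlay it binds to "Herd"-tagged actors' destruction and every BP_InsectPen's add/remove events, and creates the progress HUD.
; At milestones in the Operation map, it updates the HUD and player's progress indicator, then messages the mapped object via BPI_ProgressObject, or destroys it without that interface.
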(event `OnHerdDeath` :!signature `self.OnDestroyed`
  (params (DestroyedActor :type "Actor Object Reference"))
  (bind _result (`/Engine/EditorBlueprintResources/StandardMacros.IncrementInt` (`self.DeadCreatures`))
    (:`  `
      (`/Game/UI/WBP_HUD_progressBar.UpdateDeath` (`self.UI`) _result))))

(event `self.ReceiveBeginPlay`
  (bind _outactors (`GameplayStatics.GetAllActorsWithTag` "Herd"))
  (for _array_element _outactors
    (add `self.OnDestroyed` _array_element (delegate `OnHerdDeath`)))
  (bind _output_get (set `self.TotalCreatures` (`KismetArrayLibrary.Array_Length` _outactors)))
  (`KismetSystemLibrary.PrintString` (`KismetStringLibrary.Conv_IntToString` _output_get))
  (bind _returnvalue (`|CreateWidget` "/Game/UI/WBP_HUD_progressBar.WBP_HUD_progressBar_C" null self))
  (bind _keys (`BlueprintMapLibrary.Map_Keys` (`self.Operation`)))
  (set `self.UI` _returnvalue)
  (`UserWidget.AddToViewport` _returnvalue 0)
  (`KismetSystemLibrary.Delay` 0.2)
  (`/Game/UI/WBP_HUD_progressBar.SetIcons` _returnvalue _keys)
  (bind _outactors_2 (`GameplayStatics.GetAllActorsOfClass` "/Game/GAMEPLAY/GPE/Pen/BP_InsectPen.BP_InsectPen_C"))
  (for _array_element_2 _outactors_2
    (add `/Game/GAMEPLAY/GPE/Pen/BP_InsectPen.Added` _array_element_2 (delegate `AddCount`))
    (add `/Game/GAMEPLAY/GPE/Pen/BP_InsectPen.Removed` _array_element_2 (delegate `RemoveCount`))))

(event `AddCount`
  (bind _operation (`self.Operation`))
  (bind _creaturesgathered (`self.CreaturesGathered`))
  (bind _value (`BlueprintMapLibrary.Map_Find` _operation _creaturesgathered))
  (bind _result (`/Engine/EditorBlueprintResources/StandardMacros.IncrementInt` (`self.CreaturesGathered`))
    (:`  `
      (`KismetSystemLibrary.PrintString` (`KismetStringLibrary.Conv_IntToString` _result))
      (bind _keys (`BlueprintMapLibrary.Map_Keys` _operation))
      (if (`KismetArrayLibrary.Array_Contains` _keys _creaturesgathered)
        (`/Game/UI/WBP_HUD_progressBar.CheckOpen` (`self.UI`) _creaturesgathered _keys)
        (bind _asbp_third_person_character (cast `/Game/GAMEPLAY/PlayerCharacter/Blueprints/BP_ThirdPersonCharacter` (`GameplayStatics.GetPlayerPawn` 0)))
        (`/Game/GAMEPLAY/PlayerCharacter/Blueprints/BP_ThirdPersonCharacter.ProgressIndicator` _asbp_third_person_character (`BlueprintMapLibrary.Map_Find` (`self.OperationPoint`) _creaturesgathered))
        (if (`KismetSystemLibrary.DoesImplementInterface` _value "/Game/GAMEPLAY/INTERFACE/BPI_ProgressObject.BPI_ProgressObject_C")
          (message `/Game/GAMEPLAY/INTERFACE/BPI_ProgressObject.UnlockProgress` _value)
          (else
            (`self.K2_DestroyActor` _value)
            (`BlueprintMapLibrary.Map_Remove` (`self.Operation`) (`self.CreaturesGathered`))))))))

(event `RemoveCount`
  (bind _result (`/Engine/EditorBlueprintResources/StandardMacros.DecrementInt` (`self.CreaturesGathered`))
    (:`  `
      (`KismetSystemLibrary.PrintString` (`KismetStringLibrary.Conv_IntToString` _result)))))

(event `SmiteCreature`)

(fn `UserConstructionScript`)