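; BP_Spider is a grabbable, throwable environment object that turns into a zipline where it lands.
; On BeginPlay, a forward line trace sets the cable's anchor point.
; After a throw, a sphere hit stops physics, hides the cable, spawns a BP_zipline to that anchor and starts a countdown shown as text.
; Grabbing it removes the zipline, while timer expiry also lerps it back to the anchor through the Return timeline.
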(event `self.ReceiveTick`
  (params (DeltaSeconds :type "Float (single-precision)"))
  (bind _timerreturn (`self.TimerReturn`))
  (bind _textrender (`self.TextRender`))
  (if (`KismetSystemLibrary.K2_IsValidTimerHandle` _timerreturn)
    (`SceneComponent.SetVisibility` _textrender true false)
    (`TextRenderComponent.K2_SetText` _textrender (`KismetTextLibrary.Conv_IntToText` (`KismetMathLibrary.FFloor` (`KismetSystemLibrary.K2_GetTimerRemainingTimeHandle` _timerreturn))))
    (else
      (`SceneComponent.SetVisibility` _textrender false false))))

(event `self.ReceiveBeginPlay`
  (bind _returnvalue (`self.K2_GetActorLocation`))
  (bind _outhit (`KismetSystemLibrary.LineTraceSingle` _returnvalue (+ _returnvalue (* (`SceneComponent.GetForwardVector` (`self.Arrow`)) 100.0)) "TraceTypeQuery1"))
  (bind _output_get (set `self.InitialAttach` (`.ImpactPoint` (`GameplayStatics.BreakHitResult` _outhit))))
  (`SceneComponent.K2_SetWorldLocation` (`self.CableAttach`) _output_get false false))

(event `/Game/GAMEPLAY/INTERFACE/BPI_PlayerInteractible.ReadyThrow`
  (set `self.Thrown` true))

(event `/Game/GAMEPLAY/INTERFACE/BPI_PlayerInteractible.Grabbed`
  (bind _timerreturn (`self.TimerReturn`))
  (bind _spawnedattach (`self.SpawnedAttach`))
  (`SceneComponent.SetVisibility` (`self.Cable`) true false)
  (`/Engine/EditorBlueprintResources/StandardMacros.IsValid` _spawnedattach
    (:`Is Valid`
      (`self.K2_DestroyActor` _spawnedattach)
      (set `self.SpawnedAttach` null)
      (`KismetSystemLibrary.K2_PauseTimerHandle` _timerreturn)
      (`KismetSystemLibrary.K2_ClearAndInvalidateTimerHandle` _timerreturn))))

(event `Detach`
  (bind _spawnedattach (`self.SpawnedAttach`))
  (bind _timerreturn (`self.TimerReturn`))
  (`SceneComponent.SetVisibility` (`self.Cable`) true false)
  (`/Engine/EditorBlueprintResources/StandardMacros.IsValid` _spawnedattach
    (:`Is Valid`
      (`self.K2_DestroyActor` _spawnedattach)
      (set `self.SpawnedAttach` null)
      (set `self.CurrentAttach` (`self.K2_GetActorLocation`))
      (`KismetSystemLibrary.K2_PauseTimerHandle` _timerreturn)
      (`KismetSystemLibrary.K2_ClearAndInvalidateTimerHandle` _timerreturn)
      (bind (_direction _returnvalue) (`Timeline|Return` :!via `PlayFromStart`)
        (:`Update`
          (`self.K2_SetActorLocation` (`KismetMathLibrary.VLerp` (`self.CurrentAttach`) (`self.InitialAttach`) _returnvalue)))))))

(event `self.Sphere.OnComponentHit`
  (params (HitComponent :type "PrimitiveComponent Object Reference") (OtherActor :type "Actor Object Reference") (OtherComp :type "PrimitiveComponent Object Reference") (NormalImpulse :type "Vector Structure") (Hit :type "HitResult Structure (by ref)"))
  (if (`self.Thrown`)
    (set `self.Thrown` false)
    (`PrimitiveComponent.SetSimulatePhysics` (`self.Sphere`) false)
    (bind _returnvalue (`|SpawnActorFromClass` "/Game/GAMEPLAY/GPE/InteractibleEnvironments/BP_zipline.BP_zipline_C" (`KismetMathLibrary.MakeTransform` (`self.K2_GetActorLocation`)) "Undefined" "MultiplyWithRoot" null null))
    (`SceneComponent.SetVisibility` (`self.Cable`) false false)
    (`SceneComponent.K2_SetWorldLocation` (`/Game/GAMEPLAY/GPE/InteractibleEnvironments/BP_zipline.Endvisualized` _returnvalue) (`self.InitialAttach`) false false)
    (`/Game/GAMEPLAY/GPE/InteractibleEnvironments/BP_zipline.Initialize` _returnvalue)
    (set `self.SpawnedAttach` _returnvalue)
    (`KismetSystemLibrary.PrintString` "SetTimer")
    (bind _returnvalue_2 (`KismetSystemLibrary.K2_SetTimerDelegate` (delegate `Detach`) 20.0))
    (set `self.TimerReturn` _returnvalue_2)))

(fn `UserConstructionScript`)