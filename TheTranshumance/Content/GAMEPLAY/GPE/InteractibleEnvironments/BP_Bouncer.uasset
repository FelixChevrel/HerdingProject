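; Bounce pad environment actor that launches interacting actors along its arrow direction and can sprout into place when unlocked.
; When an actor's root component enters the box, it sends a bounce message through BPI_EnvironmentInteraction with a short delay and set power, then plays a squash timeline on the cube.
; UnlockProgress runs a sped-up Sprout timeline that scales the cube and moves the actor from its starting location by the EndGoal offset.
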(event `self.ReceiveBeginPlay`
  (set `self.InitialLock` (`self.K2_GetActorLocation`))
  (`TimelineComponent.SetPlayRate` (`self.Sprout`) 3.0))

(event `self.Box.OnComponentBeginOverlap`
  (params (OverlappedComponent :type "PrimitiveComponent Object Reference") (OtherActor :type "Actor Object Reference") (OtherComp :type "PrimitiveComponent Object Reference") (OtherBodyIndex :type Integer) (bFromSweep :type Boolean) (SweepResult :type "HitResult Structure (by ref)"))
  (if (== OtherComp (`Actor.RootComponent` OtherActor))
    (if (`KismetSystemLibrary.DoesImplementInterface` OtherActor "/Game/GAMEPLAY/INTERFACE/BPI_EnvironmentInteraction.BPI_EnvironmentInteraction_C")
      (message `/Game/GAMEPLAY/INTERFACE/BPI_EnvironmentInteraction.BOUNCE` OtherActor 0.2 (`KismetMathLibrary.Normal` (`SceneComponent.GetForwardVector` (`self.Arrow`))) (`self.Power`))
      (bind (_direction _newtrack_0) (`Timeline|Squash` :!via `PlayFromStart`)
        (:`Update`
          (`SceneComponent.SetRelativeScale3D` (`self.Cube`) (`KismetMathLibrary.MakeVector` 0.375 0.375 (* _newtrack_0 0.375))))))))

(event `/Game/GAMEPLAY/INTERFACE/BPI_ProgressObject.UnlockProgress`
  (bind (_direction _scale _location) (`Timeline|Sprout` :!via `PlayFromStart`)
    (:`Update`
      (`KismetSystemLibrary.PrintString` "Sprouting")
      (`SceneComponent.SetRelativeScale3D` (`self.Cube`) (`KismetMathLibrary.Conv_DoubleToVector` (* _scale 0.375)))
      (`self.K2_SetActorLocation` (`KismetMathLibrary.VLerp` (`self.InitialLock`) (+ (`self.InitialLock`) (`self.EndGoal`)) _location)))))

(fn `UserConstructionScript`)