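; Zipline actor that carries an attached player from its root toward an editable end point, Endvisualized.
; The construction script sizes the cable to the end point's distance, and BeginPlay computes the travel direction and stretches, centers and rotates a box along the line.
; Each Tick, when the player is attached and this is its ClosestAttach, it faces them along the line and moves them at Speed with sweep.
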(event `self.ReceiveBeginPlay`
  (`self.Initialize`))

(event `Initialize`
  (bind _relativelocation (`SceneComponent.RelativeLocation` (`self.Endvisualized`)))
  (bind _returnvalue (`KismetMathLibrary.FindLookAtRotation` (`SceneComponent.K2_GetComponentLocation` (`self.DefaultSceneRoot`)) (`SceneComponent.K2_GetComponentLocation` (`self.Endvisualized`))))
  (set `self.Direction` (`KismetMathLibrary.GetForwardVector` _returnvalue))
  (`BoxComponent.SetBoxExtent` (`self.Box`) (`KismetMathLibrary.MakeVector` (/ (`KismetMathLibrary.VSize` _relativelocation) 2.0) 10.0 10.0) true)
  (`SceneComponent.K2_SetWorldRotation` (`self.Box`) _returnvalue false false)
  (`SceneComponent.K2_SetRelativeLocation` (`self.Box`) (/ _relativelocation 2.0) false false))

(event `self.ReceiveTick`
  (params (DeltaSeconds :type "Float (single-precision)"))
  (bind _player (`self.Player`))
  (bind _player_2 (`self.Player`))
  (`/Engine/EditorBlueprintResources/StandardMacros.IsValid` _player
    (:`Is Valid`
      (if (and (`/Game/GAMEPLAY/PlayerCharacter/Blueprints/BP_ThirdPersonCharacter.OnAttach` _player) (== (`/Game/GAMEPLAY/PlayerCharacter/Blueprints/BP_ThirdPersonCharacter.ClosestAttach` _player) self))
        (`self.K2_SetActorRotation` _player_2 (`KismetMathLibrary.FindLookAtRotation` (`SceneComponent.K2_GetComponentLocation` (`self.DefaultSceneRoot`)) (`SceneComponent.K2_GetComponentLocation` (`self.Endvisualized`))) false)
        (`self.K2_AddActorWorldOffset` _player_2 (* (`self.Direction`) (`self.Speed`) DeltaSeconds) true false)))))

(fn `UserConstructionScript`
  (set `CableComponent.CableLength` (`KismetMathLibrary.VSize` (`SceneComponent.RelativeLocation` (`self.Endvisualized`))) (`self.Cable`)))