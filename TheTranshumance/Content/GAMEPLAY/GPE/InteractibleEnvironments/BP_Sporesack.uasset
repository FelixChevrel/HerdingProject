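; BP_Sporesack is a throwable environment object that turns into a bounce pad where it lands.
; On BeginPlay, a short trace along its Arrow sets the world location of its cable attach point.
; ReadyThrow arms it; the next Sphere hit stops physics, spawns a powered BP_Bouncer facing along the surface normal and destroys the sack.
; Grabbed and MarkHerd are stubs, and a debug arrow is drawn on impact.
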(event `self.ReceiveTick`
  (params (DeltaSeconds :type "Float (single-precision)")))

(event `self.ReceiveBeginPlay`
  (bind _returnvalue (`self.K2_GetActorLocation`))
  (bind _outhit (`KismetSystemLibrary.LineTraceSingle` _returnvalue (+ _returnvalue (* (`SceneComponent.GetForwardVector` (`self.Arrow`)) 100.0)) "TraceTypeQuery1"))
  (bind _output_get (set `self.InitialAttach` (`.ImpactPoint` (`GameplayStatics.BreakHitResult` _outhit))))
  (`SceneComponent.K2_SetWorldLocation` (`self.CableAttach`) _output_get false false))

(event `/Game/GAMEPLAY/INTERFACE/BPI_PlayerInteractible.ReadyThrow`
  (set `self.Thrown` true))

(event `/Game/GAMEPLAY/INTERFACE/BPI_PlayerInteractible.Grabbed`)

(event `self.Sphere.OnComponentHit`
  (params (HitComponent :type "PrimitiveComponent Object Reference") (OtherActor :type "Actor Object Reference") (OtherComp :type "PrimitiveComponent Object Reference") (NormalImpulse :type "Vector Structure") (Hit :type "HitResult Structure (by ref)"))
  (bind (_bblockinghit _binitialoverlap _time _distance _location _impactpoint _normal) (`GameplayStatics.BreakHitResult` Hit))
  (bind _returnvalue (+ _impactpoint (* _normal 100.0)))
  (if (`self.Thrown`)
    (set `self.Thrown` false)
    (`PrimitiveComponent.SetSimulatePhysics` (`self.Sphere`) false)
    (`KismetSystemLibrary.DrawDebugArrow` _impactpoint _returnvalue 10.0 (struct :`R` 0.703596 :`G` 1.0 :`A` 1.0) 10.0 3.0)
    (bind _returnvalue_2 (`|SpawnActorFromClass` "/Game/GAMEPLAY/GPE/InteractibleEnvironments/BP_Bouncer.BP_Bouncer_C" (`KismetMathLibrary.MakeTransform` _impactpoint (`KismetMathLibrary.FindLookAtRotation` _impactpoint _returnvalue) (2.0 2.0 2.0)) "Undefined" "MultiplyWithRoot" null null))
    (set `/Game/GAMEPLAY/GPE/InteractibleEnvironments/BP_Bouncer.Power` 1750.0 _returnvalue_2)
    (`self.K2_DestroyActor`)))

(fn `MarkHerd`
  (params (Player :type "/Game/GAMEPLAY/PlayerCharacter/Blueprints/BP_ThirdPersonCharacter Object Reference") (Unmark :type Boolean))
  (returns (IsHerd :type Boolean))
  (return false))

(fn `UserConstructionScript`)