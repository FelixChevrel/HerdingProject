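; Placeable gameplay helper that snaps a tagged actor to its own position and rotation when that actor enters its detection area.
; On overlap, an actor carrying the researched tag is detached, moved to the helper's transform while keeping its scale, and has its velocities zeroed.
; StopPhysic decides whether physics simulation is switched off on the snapped actor's root.
; It works once, clearing Active after the snap.
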(event `self.DetectionArea.OnComponentBeginOverlap`
  (params (OverlappedComponent :type "PrimitiveComponent Object Reference") (OtherActor :type "Actor Object Reference") (OtherComp :type "PrimitiveComponent Object Reference") (OtherBodyIndex :type Integer) (bFromSweep :type Boolean) (SweepResult :type "HitResult Structure (by ref)"))
  (if (`self.Active?`)
    (if (`self.ActorHasTag` OtherActor (`self.ResearchedTag`))
      (`self.K2_DetachFromActor` OtherActor "KeepWorld" "KeepWorld" "KeepWorld")
      (`self.K2_SetActorTransform` OtherActor (`KismetMathLibrary.MakeTransform` (`self.K2_GetActorLocation`) (`self.K2_GetActorRotation`) (`self.GetActorScale3D` OtherActor)) false false)
      (bind _asprimitive_component (cast `PrimitiveComponent` (`Actor.RootComponent` OtherActor)))
      (`PrimitiveComponent.SetSimulatePhysics` _asprimitive_component (not (`self.StopPhysic`)))
      (`PrimitiveComponent.SetPhysicsLinearVelocity` _asprimitive_component (0.0 0.0 0.0) false "None")
      (`PrimitiveComponent.SetAllPhysicsAngularVelocityInDegrees` _asprimitive_component (0.0 0.0 0.0) false)
      (set `self.Active?` false))))

(fn `UserConstructionScript`)