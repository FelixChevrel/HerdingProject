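; BP_DogBlock is a pet gameplay element that reports itself as a DogPull interaction, offering four possible spots marked by arrows.
; SetSpotLocation selects the first arrow within a scale-adjusted radius of a hit location, shows only that arrow and keeps the previous spot if none qualifies.
; Where? returns the selected arrow's first child location and the arrow's rotation as the exact placement.
; The block itself contains no movement logic.
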(event `/Game/GAMEPLAY/INTERFACE/BPI_PetInteractible.SetSpotLocation`
  (params (HitLocation :type "Vector Structure"))
  (bind _returnvalue_x (`KismetMathLibrary.BreakVector` (`self.GetActorRelativeScale3D`)))
  (bind _arrow3 (`self.Arrow3`))
  (bind _arrow1 (`self.Arrow1`))
  (bind _arrow2 (`self.Arrow2`))
  (bind _arrow (`self.Arrow`))
  (bind _returnvalue (* 112.0 _returnvalue_x))
  (if (<= (`KismetMathLibrary.Vector_Distance` HitLocation (`SceneComponent.K2_GetComponentLocation` (`self.Arrow`))) _returnvalue)
    (set `self.CurrentSpot` _arrow)
    (`SceneComponent.SetVisibility` _arrow true false)
    (`SceneComponent.SetVisibility` (`self.Arrow2`) false false)
    (`SceneComponent.SetVisibility` (`self.Arrow3`) false false)
    (`SceneComponent.SetVisibility` (`self.Arrow1`) false false)
    (elif (<= (`KismetMathLibrary.Vector_Distance` HitLocation (`SceneComponent.K2_GetComponentLocation` (`self.Arrow1`))) _returnvalue)
      (set `self.CurrentSpot` _arrow1)
      (`SceneComponent.SetVisibility` _arrow1 true false)
      (`SceneComponent.SetVisibility` (`self.Arrow2`) false false)
      (`SceneComponent.SetVisibility` (`self.Arrow3`) false false)
      (`SceneComponent.SetVisibility` (`self.Arrow`) false false)
      (elif (<= (`KismetMathLibrary.Vector_Distance` HitLocation (`SceneComponent.K2_GetComponentLocation` (`self.Arrow2`))) _returnvalue)
        (set `self.CurrentSpot` _arrow2)
        (`SceneComponent.SetVisibility` _arrow2 true false)
        (`SceneComponent.SetVisibility` (`self.Arrow1`) false false)
        (`SceneComponent.SetVisibility` (`self.Arrow`) false false)
        (`SceneComponent.SetVisibility` (`self.Arrow3`) false false)
        (elif (<= (`KismetMathLibrary.Vector_Distance` HitLocation (`SceneComponent.K2_GetComponentLocation` (`self.Arrow3`))) _returnvalue)
          (set `self.CurrentSpot` _arrow3)
          (`SceneComponent.SetVisibility` _arrow3 true false)
          (`SceneComponent.SetVisibility` (`self.Arrow1`) false false)
          (`SceneComponent.SetVisibility` (`self.Arrow`) false false)
          (`SceneComponent.SetVisibility` (`self.Arrow2`) false false))))))

(fn `AttackFeedbackData`
  (returns (HPLeft :type Integer))
  (return 0))

(fn `UserConstructionScript`)

(fn `WhatType?`
  (returns (Orders :type "actionTypes Enum"))
  (return "dogPull"))

(fn `Where?`
  (returns (SpecificSpot :type Boolean) (Coordinates :type "Vector Structure") (SpecificRot :type Boolean) (Rot :type "Rotator Structure"))
  (bind _currentspot (`self.CurrentSpot`))
  (return true (`SceneComponent.K2_GetComponentLocation` (`SceneComponent.GetChildComponent` _currentspot 0)) true (`SceneComponent.K2_GetComponentRotation` _currentspot)))