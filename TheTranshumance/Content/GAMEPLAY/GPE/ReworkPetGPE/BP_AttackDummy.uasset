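; BP_AttackDummy is a pet gameplay element that reports its type as DogAttack and serves as a physics dummy knocked around by attacks.
; Attack replaces the Dummy component's linear velocity with the attack direction scaled by attack power, while GetHit launches it along the supplied forward vector at a fixed speed.
; AttackFeedbackData only returns zero, and the actor has no active tick, overlap or construction logic.
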(event `/Game/GAMEPLAY/INTERFACE/BPI_PetInteractible.Attack`
  (params (AttackOrigin :type "Vector Structure") (AttackDirection :type "Vector Structure") (AttackPower :type "Float (double-precision)"))
  (`PrimitiveComponent.SetPhysicsLinearVelocity` (`self.Dummy`) (* AttackDirection AttackPower) false "None"))

(event `/Game/GAMEPLAY/INTERFACE/BPI_StrikeInteraction.GetHit`
  (params (Hitcoordinate :type "Vector Structure") (ForwardVector :type "Vector Structure"))
  (`PrimitiveComponent.SetPhysicsLinearVelocity` (`self.Dummy`) (* ForwardVector 1000.0) false "None"))

(fn `AttackFeedbackData`
  (returns (HPLeft :type Integer))
  (return 0))

(fn `UserConstructionScript`)

(fn `WhatType?`
  (returns (Orders :type "actionTypes Enum"))
  (return "dogAttack"))