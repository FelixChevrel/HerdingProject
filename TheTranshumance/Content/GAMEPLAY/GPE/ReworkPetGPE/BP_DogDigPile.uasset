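; BP_DogDigPile is a pet-interaction pile, typed DogDig, that can reveal a configurable object when it reacts.
; Reaction hides the cube, then spawns ObjectSpawned at the pile's location at a tiny scale, if that class is valid.
; The SpawnEffect timeline scales the spawned actor uniformly, and the pile destroys itself when it finishes.
; With no valid class, the pile is destroyed immediately.
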(event `/Game/GAMEPLAY/INTERFACE/BPI_PetInteractible.Reaction`
  (`SceneComponent.SetVisibility` (`self.Cube`) false false)
  (if (`KismetSystemLibrary.IsValidClass` (`self.ObjectSpawned`))
    (bind _returnvalue (`|SpawnActorFromClass` (`self.ObjectSpawned`) (`KismetMathLibrary.MakeTransform` (`self.K2_GetActorLocation`) (struct) (0.1 0.1 0.1)) "AlwaysSpawn" "MultiplyWithRoot" null null))
    (set `self.SpawnedEntity` _returnvalue)
    (bind (_direction _newtrack_0) (`Timeline|SpawnEffect`)
      (:`Update`
        (`self.SetActorScale3D` (`self.SpawnedEntity`) (`KismetMathLibrary.MakeVector` _newtrack_0 _newtrack_0 _newtrack_0)))
      (:`Finished`
        (`self.K2_DestroyActor`)))
    (else
      (`self.K2_DestroyActor`))))

(fn `AttackFeedbackData`
  (returns (HPLeft :type Integer))
  (return 0))

(fn `UserConstructionScript`)

(fn `WhatType?`
  (returns (Orders :type "actionTypes Enum"))
  (return "dogDig"))