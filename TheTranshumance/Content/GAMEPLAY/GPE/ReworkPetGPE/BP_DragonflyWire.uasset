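; BP_DragonflyWire is a pet gameplay element: a wire holding Cube1 that can be cut through a DragCut interaction.
; Tick keeps Sphere at the midpoint between Cube and Cube1, and Where? reports that point as the interaction spot.
; Reaction destroys the constraint, cable and Sphere and nudges Cube1 downward.
; When Cube1 registers a hit and HasLoot is set, it spawns Loot in its place and destroys itself.
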(event `self.ReceiveTick`
  (params (DeltaSeconds :type "Float (single-precision)"))
  (bind _sphere (`self.Sphere`))
  (bind _returnvalue (`SceneComponent.K2_GetComponentLocation` (`self.Cube1`)))
  (`/Engine/EditorBlueprintResources/StandardMacros.IsValid` _sphere
    (:`Is Valid`
      (`SceneComponent.K2_SetWorldLocation` _sphere (+ _returnvalue (/ (- (`SceneComponent.K2_GetComponentLocation` (`self.Cube`)) _returnvalue) 2.0)) false false))))

(event `/Game/GAMEPLAY/INTERFACE/BPI_PetInteractible.Reaction`
  (`ActorComponent.K2_DestroyComponent` (`self.PhysicsConstraint`))
  (`ActorComponent.K2_DestroyComponent` (`self.Cable`))
  (`PrimitiveComponent.AddImpulse` (`self.Cube1`) (0.0 0.0 -5.0) "None" false)
  (`ActorComponent.K2_DestroyComponent` (`self.Sphere`)))

(event `self.Cube1.OnComponentHit`
  (params (HitComponent :type "PrimitiveComponent Object Reference") (OtherActor :type "Actor Object Reference") (OtherComp :type "PrimitiveComponent Object Reference") (NormalImpulse :type "Vector Structure") (Hit :type "HitResult Structure (by ref)"))
  (bind _cube1 (`self.Cube1`))
  (if (`self.HasLoot`)
    (`|SpawnActorFromClass` (`self.loot`) (`KismetMathLibrary.MakeTransform` (`SceneComponent.K2_GetComponentLocation` _cube1) (`SceneComponent.K2_GetComponentRotation` _cube1)) "AlwaysSpawn" "MultiplyWithRoot" null null)
    (`ActorComponent.K2_DestroyComponent` _cube1)))

(fn `AttackFeedbackData`
  (returns (HPLeft :type Integer))
  (return 0))

(fn `UserConstructionScript`)

(fn `WhatType?`
  (returns (Orders :type "actionTypes Enum"))
  (return "dragCut"))

(fn `Where?`
  (returns (SpecificSpot :type Boolean) (Coordinates :type "Vector Structure") (SpecificRot :type Boolean) (Rot :type "Rotator Structure"))
  (return true (`SceneComponent.K2_GetComponentLocation` (`self.Sphere`)) false))